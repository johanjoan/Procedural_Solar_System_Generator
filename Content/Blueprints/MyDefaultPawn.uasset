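; Default pawn Blueprint that shows a velocity HUD and handles opening the pause menu.
; On BeginPlay it adds the UI_Velocity widget to the viewport.
; Escape calls PauseGame, which creates W_PauseMenu, pauses the game and switches to Game and UI input with a cursor.
; An unpause branch reverses this, but IsGamePaused is set false in both branches, so this graph never sets up that toggle.
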(event `PauseGame`
  (bind _returnvalue (`GameplayStatics.GetPlayerController` 0))
  (if (not (`self.isGamePaused?`))
    (set `self.isGamePaused?` false)
    (bind _returnvalue_2 (`|CreateWidget` "/Game/Blueprints/W_PauseMenu.W_PauseMenu_C" _returnvalue))
    (bind _output_get (set `self.PauseMenuWidget` _returnvalue_2))
    (`UserWidget.AddToViewport` _output_get 0)
    (`WidgetBlueprintLibrary.SetInputMode_GameAndUIEx` _returnvalue (`self.PauseMenuWidget`))
    (set `PlayerController.bShowMouseCursor` true (`GameplayStatics.GetPlayerController` 0))
    (`GameplayStatics.SetGamePaused` true)
    (else
      (set `self.isGamePaused?` false)
      (`Widget.RemoveFromParent` (`self.PauseMenuWidget`))
      (`GameplayStatics.SetGamePaused` false)
      (`WidgetBlueprintLibrary.SetInputMode_GameOnly` _returnvalue)
      (set `PlayerController.bShowMouseCursor` false (`GameplayStatics.GetPlayerController` 0)))))

(event `self.ReceiveBeginPlay`
  (bind _returnvalue (`|CreateWidget` "/Game/Blueprints/UI_Velocity.UI_Velocity_C"))
  (`UserWidget.AddToViewport` _returnvalue 0))

(event `Key|Escape`
  (params (Key :type "Key Structure"))
  (:`Pressed`
    (`self.PauseGame`)))

(event `self.ReceiveTick`
  (params (DeltaSeconds :type "Float (single-precision)")))

(fn `UserConstructionScript`)